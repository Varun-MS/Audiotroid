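; Music-reactive enemy that moves steadily along negative Y each tick and is destroyed on overlapping a DeSpawner.
; Construction creates a dynamic sphere material and caches the first EQControllerLower, whose BassTempo drives the clamped Intensity parameter every tick.
; On Hit, high Intensity makes it explode with a sound; otherwise it spawns two copies at 0.5 scale in its place.
; Movement is frame-rate dependent, and Tick prints Intensity for debugging.
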(event `self.ReceiveTick`
  (params (DeltaSeconds :type "Float (single-precision)"))
  (bind _enemymaterial (`self.EnemyMaterial`))
  (`self.K2_SetActorLocation` (+ (`self.K2_GetActorLocation`) (0.0 -6.0 0.0) (0.0 0.0 0.0)))
  (bind _returnvalue (`MaterialInstanceDynamic.K2_GetScalarParameterValue` _enemymaterial "Intensity"))
  (`KismetSystemLibrary.PrintString` (`KismetStringLibrary.Conv_DoubleToString` _returnvalue))
  (`MaterialInstanceDynamic.SetScalarParameterValue` _enemymaterial "Intensity" (`KismetMathLibrary.FClamp` (/ (`/Game/EQControllerLower.BassTempo` (`self.BassTempoReference`)) 3.0) 1.0 15.0)))

(event `self.ReceiveActorBeginOverlap`
  (params (OtherActor :type "Actor Object Reference"))
  (cast `/Game/Blueprints/DeSpawner` OtherActor)
  (`self.K2_DestroyActor`))

(event `Hit`
  (bind _returnvalue (`KismetMathLibrary.MakeTransform` (.location (`self.GetTransform`)) (.rotation (`self.GetTransform`)) (0.5 0.5 0.5)))
  (bind _returnvalue_2 (`MaterialInstanceDynamic.K2_GetScalarParameterValue` (`self.EnemyMaterial`) "Intensity"))
  (if (>= _returnvalue_2 9.0)
    (`GameplayStatics.PlaySoundAtLocation` "/Game/Data/Explosion01.Explosion01" (`self.K2_GetActorLocation`))
    (`self.K2_DestroyActor`)
    (else
      (`|SpawnActorFromClass` "EnemyBlueprint_C" _returnvalue "Undefined" "OverrideRootScale" null null)
      (`|SpawnActorFromClass` "EnemyBlueprint_C" _returnvalue "Undefined" "OverrideRootScale" null null)
      (`self.K2_DestroyActor`))))

(fn `UserConstructionScript`
  (bind _returnvalue (`PrimitiveComponent.CreateDynamicMaterialInstance` (`self.Sphere`) 1 null))
  (set `self.EnemyMaterial` _returnvalue)
  (bind _outactors (`GameplayStatics.GetAllActorsOfClass` "/Game/EQControllerLower.EQControllerLower_C"))
  (set `self.BassTempoReference` (`|GetArrayItem` _outactors)))