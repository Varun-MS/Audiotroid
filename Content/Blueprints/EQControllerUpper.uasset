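; EQControllerUpper drives an audio visualizer, scaling a row of EQBarUpper actors to a sound's frequency spectrum.
; BeginPlay gathers the bars and insertion-sorts them by descending Y position so array index maps to frequency band.
; Each Tick samples a short spectrum window slightly ahead of game time and sets each bar's Z scale from its clamped, cubed value.
; Audio playback nodes exist but are disconnected.
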(event `self.ReceiveBeginPlay`
  (bind _eqbarupper (`self.EQBarUpper`))
  (bind _outactors (`GameplayStatics.GetAllActorsOfClass` "/Game/EQBarUpper.EQBarUpper_C"))
  (for _array_element _outactors
    (for (_array_element_2 _array_index) _eqbarupper
      (if (not (> (.y (`self.K2_GetActorLocation` _array_element_2)) (.y (`self.K2_GetActorLocation` _array_element))))
        (break)))
    (`KismetArrayLibrary.Array_Insert` _eqbarupper _array_element _array_index)))

(event `self.ReceiveTick`
  (params (DeltaSeconds :type "Float (single-precision)"))
  (bind _outspectrum (`SoundVisualizationStatics.CalculateFrequencySpectrum` (`self.SOUND`) 0 (+ (`KismetSystemLibrary.GetGameTimeInSeconds`) 0.11) 0.22 30))
  (set `self.Frequencies` _outspectrum)
  (for (_array_element _array_index) (`self.EQBarUpper`)
    (bind _returnvalue (`KismetMathLibrary.FClamp` (/ (`|GetArrayItem` (`self.Frequencies`) _array_index) 17.5) 0.0 2.5))
    (`self.SetActorScale3D` _array_element (`KismetMathLibrary.MakeVector` 0.9 1.5 (+ (* _returnvalue _returnvalue _returnvalue) 0.1)))))

(fn `UserConstructionScript`)