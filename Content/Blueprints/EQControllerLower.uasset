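; Audio visualizer controller that plays a sound and animates a row of EQBarLower actors as equalizer bars.
; On BeginPlay it insertion-sorts the bars by Y position and starts the audio inside that same loop.
; Each Tick samples the sound's frequency spectrum slightly ahead of game time, scaling each bar's height by its cubed, clamped band value.
; The lowest band is stored as BassTempo; a threshold debug print is left unconnected.
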(event `self.ReceiveBeginPlay`
  (bind _audio (`self.Audio`))
  (bind _eqbarlower (`self.EQBarLower`))
  (bind _outactors (`GameplayStatics.GetAllActorsOfClass` "/Game/EQBarLower.EQBarLower_C"))
  (for _array_element _outactors
    (for (_array_element_2 _array_index) _eqbarlower
      (if (not (< (.y (`self.K2_GetActorLocation` _array_element_2)) (.y (`self.K2_GetActorLocation` _array_element))))
        (break)))
    (`KismetArrayLibrary.Array_Insert` _eqbarlower _array_element _array_index)
    (`AudioComponent.SetSound` _audio (`self.SOUND`))
    (`AudioComponent.Play` _audio 0.0)))

(event `self.ReceiveTick`
  (params (DeltaSeconds :type "Float (single-precision)"))
  (bind _frequencies (`self.Frequencies`))
  (bind _outspectrum (`SoundVisualizationStatics.CalculateFrequencySpectrum` (`self.SOUND`) 0 (+ (`KismetSystemLibrary.GetGameTimeInSeconds`) 0.11) 0.22 30))
  (set `self.Frequencies` _outspectrum)
  (for (_array_element _array_index) (`self.EQBarLower`)
    (bind _returnvalue (`KismetMathLibrary.FClamp` (/ (`|GetArrayItem` _frequencies _array_index) 17.5) 0.0 2.5))
    (`self.SetActorScale3D` _array_element (`KismetMathLibrary.MakeVector` 0.9 1.5 (+ (* _returnvalue _returnvalue _returnvalue) 0.1)))
    (set `self.BassTempo` (`|GetArrayItem` _frequencies))))

(fn `UserConstructionScript`)