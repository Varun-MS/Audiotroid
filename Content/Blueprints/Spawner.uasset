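; Spawner actor that continuously spawns EnemyBlueprint actors at random points inside its SpawnArea box.
; BeginPlay starts a looping timer that fires the SpawnEnemy event at a rate set by EnemiesPerSecond.
; Each spawn picks a random point from the box's world location and scaled extent.
; BeginPlay also sets the Spawner variable on the first Spawner actor found to None.
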(event `SpawnEnemy`
  (bind _spawnarea (`self.SpawnArea`))
  (`|SpawnActorFromClass` "/Game/Blueprints/EnemyBlueprint.EnemyBlueprint_C" (`KismetMathLibrary.Conv_VectorToTransform` (`KismetMathLibrary.RandomPointInBoundingBox` (`SceneComponent.K2_GetComponentLocation` _spawnarea) (`BoxComponent.GetScaledBoxExtent` _spawnarea))) "Undefined" "OverrideRootScale" null null))

(event `self.ReceiveBeginPlay`
  (bind _outactors (`GameplayStatics.GetAllActorsOfClass` "Spawner_C"))
  (set `/Game/Blueprints/Spawner.Spawner` null (`|GetArrayItem` _outactors))
  (`KismetSystemLibrary.K2_SetTimerDelegate` (delegate `SpawnEnemy`) (/ 1.0 (`self.EnemiesPerSecond`)) true))

(fn `UserConstructionScript`)