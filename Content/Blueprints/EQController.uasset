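; EQController drives an audio equalizer visualizer built from EQBar actors placed in the level.
; On BeginPlay it insertion-sorts the bars by X position and starts the sound, re-triggering playback for each bar inserted.
; Each Tick it computes a frequency spectrum of the sound at a slight offset from game time.
; Each band's clamped, squared value sets its bar's Z scale, with raw values printed for debugging.
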(event `self.ReceiveBeginPlay`
  (bind _audio (`self.Audio`))
  (bind _eqbar (`self.EQBar`))
  (bind _outactors (`GameplayStatics.GetAllActorsOfClass` "/Game/Blueprints/EQBar.EQBar_C"))
  (for _array_element _outactors
    (for (_array_element_2 _array_index) _eqbar
      (if (not (< (.x (`self.K2_GetActorLocation` _array_element_2)) (.x (`self.K2_GetActorLocation` _array_element))))
        (break)))
    (`KismetArrayLibrary.Array_Insert` _eqbar _array_element _array_index)
    (`AudioComponent.SetSound` _audio (`self.SOUND`))
    (`AudioComponent.Play` _audio 0.0)))

(event `self.ReceiveTick`
  (params (DeltaSeconds :type "Float (single-precision)"))
  (bind _outspectrum (`SoundVisualizationStatics.CalculateFrequencySpectrum` (`self.SOUND`) 0 (+ (`KismetSystemLibrary.GetGameTimeInSeconds`) 0.11) 0.22 32))
  (set `self.Frequencies` _outspectrum)
  (for (_array_element _array_index) (`self.EQBar`)
    (bind _output (`|GetArrayItem` (`self.Frequencies`) _array_index))
    (`KismetSystemLibrary.PrintString` (`KismetStringLibrary.Conv_DoubleToString` _output))
    (bind _returnvalue (`KismetMathLibrary.FClamp` (/ _output 25.0) 0.0 5000.0))
    (`self.SetActorScale3D` _array_element (`KismetMathLibrary.MakeVector` 0.9 0.9 (+ (* _returnvalue _returnvalue 1.0) 0.1)))))

(fn `UserConstructionScript`)